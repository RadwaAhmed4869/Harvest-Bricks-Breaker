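; Base brick for a ball-bouncing brick breaker, with a hit-number widget and a randomized mesh scale and rotation.
; Each ball hit plays sound and particles, increments the Game Instance score, and decrements hit points.
; The final hit disables collision, updates the Game Mode brick count, spawns a potion if a random roll exceeds Chance, then destroys the brick.
; A Game Mode test flag auto-breaks bricks after a random delay.
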(event `self.ReceiveBeginPlay`
  ;[1 1 1] Set BrickRef for HitNumberWidget
  (bind _returnvalue (`|CreateWidget` "/Game/Radwa/Blueprints/HUD/WBP_BrickHitNumber.WBP_BrickHitNumber_C"))
  (set `/Game/Radwa/Blueprints/HUD/WBP_BrickHitNumber.BrickRef` self _returnvalue)
  (`WidgetComponent.SetWidget` (`self.HitNumberWidget`) _returnvalue)
  ;[1 1 1] Disable UI Shadow
  (`PrimitiveComponent.SetCastShadow` (`self.HitNumberWidget`) false)
  ;[1 1 1] Game Mode Ref
  (bind _ascustom_game_mode (cast `/Game/Radwa/Blueprints/CustomGameMode` (`GameplayStatics.GetGameMode`)))
  (set `self.GameModeRef` _ascustom_game_mode)
  ;[1 1 1] Game Instance Ref
  (bind _asgi_bounce (cast `/Game/Radwa/Blueprints/GI_Bounce` (`GameplayStatics.GetGameInstance`)))
  (set `self.GameInstanceRef` _asgi_bounce)
  (`self.SetRandomScale`)
  (`self.SetRandomRotation`)
  ;[0.7379 0.4397 0.2122] If Auto Destroy is Enabled, Wait few seconds then destroy self (For Testing)
  (if (`/Game/Radwa/Blueprints/CustomGameMode.T_AutoDestroy` (`self.GameModeRef`))
    (`KismetSystemLibrary.Delay` (`KismetMathLibrary.RandomFloatInRange` 5.0 20.0))
    (set `self.HitPoints` 1)
    (`/Game/Radwa/Blueprints/Interfaces/I_BallHit.Hit by Ball`)))

(event `/Game/Radwa/Blueprints/Interfaces/I_BallHit.Hit by Ball`
  (`GameplayStatics.PlaySound2D` "/Game/Radwa/Sounds/BrickBreak.BrickBreak" 0.3 (`KismetMathLibrary.RandomFloatInRange` 1.1 0.9) 0.0 null null false)
  (`GameplayStatics.SpawnEmitterAtLocation` (`self.HitEffect`) (`self.K2_GetActorLocation`))
  (`/Engine/EditorBlueprintResources/StandardMacros.IncrementInt` (`/Game/Radwa/Blueprints/GI_Bounce.PlayerScore` (`self.GameInstanceRef`))
    (:`  `
      (if (<= (`self.HitPoints`) 1)
        (`PrimitiveComponent.SetCollisionEnabled` (`self.StaticMesh`) "NoCollision")
        (`/Game/Radwa/Blueprints/CustomGameMode.DecrementBricksCount` (`self.GameModeRef`))
        (`self.SpawnPotion`)
        (`KismetSystemLibrary.Delay` 0.2)
        (`self.K2_DestroyActor`)
        (else
          (`/Engine/EditorBlueprintResources/StandardMacros.DecrementInt` (`self.HitPoints`)))))))

(fn `SetRandomRotation`
  (bind _randomangle (`self.RandomAngle`))
  (set `self.RandomAngle` (`KismetMathLibrary.RandomFloatInRange` (* (`self.RotateAngleLimit`) -1.0) (`self.RotateAngleLimit`)))
  (`SceneComponent.K2_SetRelativeRotation` (`self.StaticMesh`) (`KismetMathLibrary.MakeRotator` _randomangle 0.0 (+ _randomangle 90.0)) false false))

(fn `SetRandomScale`
  (bind _randomscale (`self.RandomScale`))
  (set `self.RandomScale` (`KismetMathLibrary.RandomFloatInRange` (`self.MinScale`) (`self.MaxScale`)))
  (`SceneComponent.SetRelativeScale3D` (`self.StaticMesh`) (`KismetMathLibrary.MakeVector` _randomscale _randomscale _randomscale)))

(fn `SpawnPotion`
  (if (> (`KismetMathLibrary.RandomFloatInRange` 0.0 1.0) (`self.Chance`))
    (`|SpawnActorFromClass` "/Game/Radwa/Blueprints/BP_Base_Potion.BP_Base_Potion_C" (`KismetMathLibrary.MakeTransform` (`self.K2_GetActorLocation`)) "Undefined" "OverrideRootScale" null null)))

(fn `UserConstructionScript`)