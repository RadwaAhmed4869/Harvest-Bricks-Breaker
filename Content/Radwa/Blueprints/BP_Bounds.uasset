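; BP_Bounds is a trigger volume that detects when the ball goes out of play in a paddle-and-ball game.
; On BeginPlay it caches the player's BP_Paddle pawn and the CustomGameMode.
; When a BP_Ball overlaps its Box component, it decrements the paddle's lives and sets the game mode's state to a new enum value.
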(event `self.ReceiveBeginPlay`
  (bind _asbp_paddle (cast `/Game/Radwa/Blueprints/BP_Paddle` (`GameplayStatics.GetPlayerPawn` 0)))
  (set `self.PaddleRef` _asbp_paddle)
  (bind _ascustom_game_mode (cast `/Game/Radwa/Blueprints/CustomGameMode` (`GameplayStatics.GetGameMode`)))
  (set `self.GameModeRef` _ascustom_game_mode))

(event `self.Box.OnComponentBeginOverlap`
  (params (OverlappedComponent :type "PrimitiveComponent Object Reference") (OtherActor :type "Actor Object Reference") (OtherComp :type "PrimitiveComponent Object Reference") (OtherBodyIndex :type Integer) (bFromSweep :type Boolean) (SweepResult :type "HitResult Structure (by ref)"))
  (cast `/Game/Radwa/Blueprints/BP_Ball` OtherActor)
  (`/Game/Radwa/Blueprints/BP_Paddle.DecrementLives` (`self.PaddleRef`))
  (`/Game/Radwa/Blueprints/CustomGameMode.SetGameState` (`self.GameModeRef`) "NewEnumerator2"))

(fn `UserConstructionScript`)