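; GI_Bounce is a Bounce game instance, going by its name, that holds the player score and handles progression between numbered levels.
; ChangeLevel increments CurrentLevel, builds the map name through GetCurrentLevelName and opens it, or opens the credits level when CurrentLevel already equals MaxLevel.
; It returns whether CurrentLevel equals MaxLevel, and a separate ResetScore function zeroes PlayerScore.
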(fn `ChangeLevel`
  (returns (`FinalLevel?` :type Boolean))
  (bind _returnvalue (== (`self.CurrentLevel`) (`self.MaxLevel`)))
  (if _returnvalue
    (set `self.Level Name` "Level-Credits")
    (else
      (`/Engine/EditorBlueprintResources/StandardMacros.IncrementInt` (`self.CurrentLevel`)
        (:`  `
          (bind _levelname (`self.GetCurrentLevelName`))
          (set `self.Level Name` _levelname)))))
  (`GameplayStatics.OpenLevel` (`self.Level Name`))
  (return _returnvalue))

(fn `GetCurrentLevelName`
  (returns (LevelName :type Name))
  (return (`KismetStringLibrary.Conv_StringToName` (`KismetStringLibrary.Concat_StrStr` "Level-" (`KismetStringLibrary.Conv_IntToString` (`self.CurrentLevel`))))))

(fn `ResetScore`
  (set `self.PlayerScore` 0))