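; Game mode for a brick-breaker game that runs match flow as an enum state machine, from Ready through Countdown and Playing to level or game end.
; SetGameState handles each transition, using delays and paddle lives to choose between retry and Game Over, while Tick drives the countdown text.
; It counts bricks at start; clearing them triggers Level Completed, which calls the game instance to change level.
; A pre-created Play Again widget appears on Game Over or Congrats.
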(event `self.ReceiveBeginPlay`
  ;[1 1 1] Ready State at the Begining
  (set `self.TheGameState` "NewEnumerator0")
  ;[1 1 1] Paddle Ref
  (bind _asbp_paddle (cast `/Game/Radwa/Blueprints/BP_Paddle` (`GameplayStatics.GetPlayerPawn` 0)))
  (set `self.PaddleRef` _asbp_paddle)
  ;[1 1 1] Game Instance Ref
  (bind _asgi_bounce (cast `/Game/Radwa/Blueprints/GI_Bounce` (`GameplayStatics.GetGameInstance`)))
  (set `self.GameInstanceRef` _asgi_bounce)
  ;[1 1 1] Set Bricks Count
  (bind _outactors (`GameplayStatics.GetAllActorsOfClass` "/Game/Radwa/Blueprints/BP_BaseBrick.BP_BaseBrick_C"))
  (set `self.BricksCount` (`KismetArrayLibrary.Array_Length` _outactors))
  ;[1 1 1] Play Again Widget
  (bind _returnvalue (`|CreateWidget` "/Game/Radwa/Blueprints/HUD/WBP_PlayAgain.WBP_PlayAgain_C"))
  (set `self.NewGameWidget` _returnvalue))

(event `self.ReceiveTick`
  (params (DeltaSeconds :type "Float (single-precision)"))
  (`|ExecutionSequence`
    (:`then_0`
      (if (`|EnumEquality` (`self.TheGameState`) "NewEnumerator1")
        (bind _output_get (set `self.CountdownNumber` (- (`self.CountdownNumber`) DeltaSeconds)))
        (if (>= _output_get 2.0)
          (set `self.CountText` "3")
          (elif (>= _output_get 1.0)
            (set `self.CountText` "2")
            (elif (>= _output_get 0.0)
              (set `self.CountText` "1")
              (else
                (`self.SetGameState` "NewEnumerator5")))))))
    (:`then_2`
      (if (`|EnumEquality` (`self.TheGameState`) "NewEnumerator6")
        (set `self.CountText` "")))))

(event `SetGameState`
  (params (GameState :type "/Game/Radwa/Blueprints/Enums/E_GameStates Enum" :default "NewEnumerator0"))
  (bind _output_get (set `self.TheGameState` GameState))
  (switch `/Game/Radwa/Blueprints/Enums/E_GameStates` _output_get
    (:`NewEnumerator0`
      (`self.ResetPlaying`))
    (:`NewEnumerator1`
      (set `self.CountdownNumber` 3.0))
    (:`NewEnumerator2`
      ;[1 1 1] Opps
      (`KismetSystemLibrary.Delay` 1.5)
      (if (>= (`/Game/Radwa/Blueprints/BP_Paddle.BallLives` (`self.PaddleRef`)) 0)
        (`self.SetGameState` "NewEnumerator0")
        (else
          (`self.SetGameState` "NewEnumerator3"))))
    (:`NewEnumerator3`
      (`KismetSystemLibrary.Delay` 2.2)
      (`self.AskPlayAgain`))
    (:`NewEnumerator4`
      (`KismetSystemLibrary.Delay` 2.2)
      (bind _finallevel_ (`/Game/Radwa/Blueprints/GI_Bounce.ChangeLevel` (`self.GameInstanceRef`)))
      (if _finallevel_
        (`KismetSystemLibrary.PrintString` "Hello")
        (`self.SetGameState` "NewEnumerator7")
        (`self.AskPlayAgain`)))
    (:`NewEnumerator5`
      (set `self.CountText` ""))))

(fn `AskPlayAgain`
  (`UserWidget.AddToViewport` (`self.NewGameWidget`) 0)
  (set `PlayerController.bShowMouseCursor` true (`GameplayStatics.GetPlayerController` 0)))

(fn `DecrementBricksCount`
  (bind _result (`/Engine/EditorBlueprintResources/StandardMacros.DecrementInt` (`self.BricksCount`))
    (:`  `
      (if (<= _result 0)
        (`GameplayStatics.PlaySound2D` null 1.0 1.0 0.0 null null)
        (`self.SetGameState` "NewEnumerator4")))))

(fn `UserConstructionScript`)