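; Ball actor for a paddle-and-ball game that moves in XY, bouncing off surfaces and notifying hit actors via I_BallHit.
; Tick moves it with a swept offset during one game state and reflects Direction on the impact normal.
; Paddle bounces add paddle input to Y and an X bias, then scale by MinSpeedFactor.
; The game mode's reset event repositions it beside the paddle with a randomized direction.
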(event `self.ReceiveBeginPlay`
  ;[1 1 1] Paddle Ref
  (set `self.PaddleRef` (cast `/Game/Radwa/Blueprints/BP_Paddle` (`GameplayStatics.GetPlayerPawn` 0) :!pure true))
  ;[1 1 1] Game Mode Ref
  (bind _ascustom_game_mode (cast `/Game/Radwa/Blueprints/CustomGameMode` (`GameplayStatics.GetGameMode`)))
  (bind _output_get (set `self.GameModeRef` _ascustom_game_mode))
  ;[1 1 1] StartPlaying is an event in Custom Game Mode
  (add `/Game/Radwa/Blueprints/CustomGameMode.ResetPlaying` _output_get (delegate `BallStartPlaying`)))

(event `BallStartPlaying`
  ;[1 1 1] StartPlaying is an event in Custom Game Mode
  (`self.ResetBallPosition`))

(event `self.ReceiveTick`
  (params (DeltaSeconds :type "Float (single-precision)"))
  (bind (_returnvalue_x _returnvalue_y) (`KismetMathLibrary.BreakVector` (* (`self.Direction`) (`self.BallSpeed`))))
  (if (`|EnumEquality` (`/Game/Radwa/Blueprints/CustomGameMode.TheGameState` (`self.GameModeRef`)) "NewEnumerator5")
    (bind _sweephitresult (`self.K2_AddActorWorldOffset` (`KismetMathLibrary.MakeVector` _returnvalue_x _returnvalue_y) true))
    (bind _asbp_paddle (cast `/Game/Radwa/Blueprints/BP_Paddle` (`.HitActor` (`GameplayStatics.BreakHitResult` _sweephitresult)))
      (:`then`
        (bind _returnvalue (`KismetMathLibrary.GetReflectionVector` (`self.Direction`) (`.ImpactNormal` (`GameplayStatics.BreakHitResult` _sweephitresult))))
        (bind (_returnvalue_x_2 _returnvalue_y_2) (`KismetMathLibrary.BreakVector` (`KismetMathLibrary.Normal` (`KismetMathLibrary.MakeVector` (.x _returnvalue) (+ (.y _returnvalue) (* (`/Game/Radwa/Blueprints/BP_Paddle.Action Value` _asbp_paddle) 10.0))) 0.001)))
        (bind _output_get (set `self.Direction` (* (`KismetMathLibrary.Normal` (`KismetMathLibrary.MakeVector` (+ _returnvalue_x_2 (`self.MinX`)) _returnvalue_y_2) 0.01) (`self.MinSpeedFactor`)))))
      (:`CastFailed`
        (set `self.Direction` _returnvalue)
        (if (`KismetSystemLibrary.DoesImplementInterface` (`.HitActor` (`GameplayStatics.BreakHitResult` _sweephitresult)) "/Game/Radwa/Blueprints/Interfaces/I_BallHit.I_BallHit_C")
          (message `/Game/Radwa/Blueprints/Interfaces/I_BallHit.Hit by Ball` (`.HitActor` (`GameplayStatics.BreakHitResult` _sweephitresult))))))))

(fn `ResetBallPosition`
  (bind (_returnvalue_x _returnvalue_y _returnvalue_z) (`KismetMathLibrary.BreakVector` (`self.K2_GetActorLocation` (`self.PaddleRef`))))
  (`self.K2_SetActorLocation` (`KismetMathLibrary.MakeVector` (+ _returnvalue_x (`self.OffsetX`)) _returnvalue_y _returnvalue_z))
  (bind _output_get (set `self.Direction` (`KismetMathLibrary.Normal` (`KismetMathLibrary.MakeVector` 14.0 (`KismetMathLibrary.RandomFloatInRange` -1.0 10.0)) 0.001))))

(fn `UserConstructionScript`)