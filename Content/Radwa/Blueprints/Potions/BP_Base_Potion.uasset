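; Base potion pickup that travels along negative X and can be collected by the paddle.
; A self-calling Delay loop started on BeginPlay applies randomized yaw spin and movement instead of using Tick.
; Paddle overlap sends a collected message to the potion target, disables collision, plays a hit sound and particle effect, then destroys the potion.
; The game mode is cached, but its state check is never executed.
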(event `self.ReceiveBeginPlay`
  ;[1 1 1] Game Mode Ref
  (bind _ascustom_game_mode (cast `/Game/Radwa/Blueprints/CustomGameMode` (`GameplayStatics.GetGameMode`)))
  (set `self.Game Mode Ref` _ascustom_game_mode)
  (`self.MoveAndRotate`))

(event `MoveAndRotate`
  (bind _returnvalue (`KismetMathLibrary.RandomFloatInRange` -7.0 -5.0))
  (`self.K2_AddActorWorldRotation` (`KismetMathLibrary.MakeRotator` 0.0 0.0 _returnvalue))
  (`self.K2_AddActorWorldOffset` (`KismetMathLibrary.MakeVector` _returnvalue))
  (`KismetSystemLibrary.Delay` 0.05)
  (`self.MoveAndRotate`))

(event `self.Box.OnComponentBeginOverlap`
  (params (OverlappedComponent :type "PrimitiveComponent Object Reference") (OtherActor :type "Actor Object Reference") (OtherComp :type "PrimitiveComponent Object Reference") (OtherBodyIndex :type Integer) (bFromSweep :type Boolean) (SweepResult :type "HitResult Structure (by ref)"))
  (cast `/Game/Radwa/Blueprints/BP_Paddle` OtherActor)
  (message `/Game/Radwa/Blueprints/Interfaces/I_PotionCollect.PotionCollected` (`self.PosionTarget`) self)
  (`PrimitiveComponent.SetCollisionEnabled` (`self.Box`) "NoCollision")
  (`GameplayStatics.PlaySound2D` "/Game/Radwa/Sounds/BrickHit.BrickHit" 0.5 1.0 0.0 null null false)
  (`GameplayStatics.SpawnEmitterAtLocation` "/Game/InfinityBladeEffects/Effects/FX_Mobile/Impacts/P_Impact_Shield_Fire.P_Impact_Shield_Fire" (`self.K2_GetActorLocation`))
  (`KismetSystemLibrary.Delay` 0.2)
  (`self.K2_DestroyActor`))

(fn `UserConstructionScript`)