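; BP_Paddle is a player-controlled paddle that slides left and right along the Y axis and keeps a ball-lives count.
; BeginPlay adds the Enhanced Input mapping, caches the custom game mode and derives a symmetric border limit from the mesh's Y scale.
; Move input offsets the paddle only in one specific game state, blocking further movement outward past either border.
; DecrementLives lowers the count, printing a death message once it is negative.
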(event `self.ReceiveBeginPlay`
  (bind _asplayer_controller (cast `PlayerController` (`self.GetController`)))
  (bind _returnvalue (pcsubsystem `EnhancedInputLocalPlayerSubsystem` _asplayer_controller))
  (`/Engine/EditorBlueprintResources/StandardMacros.IsValid` _returnvalue
    (:`Is Valid`
      (`EnhancedInputSubsystemInterface.AddMappingContext` _returnvalue "/Game/Radwa/Inputs/IMC_PaddleMapping.IMC_PaddleMapping" 0 (struct))
      (bind _ascustom_game_mode (cast `/Game/Radwa/Blueprints/CustomGameMode` (`GameplayStatics.GetGameMode`)))
      (set `self.GameModeRef` _ascustom_game_mode)
      (`self.SetBorderLimitRelativeToMeshScale`))))

(event `EnhancedInput|/Game/Radwa/Inputs/IA_MoveLeftRight`
  (params (ActionValue :type "Float (double-precision)") (ElapsedSeconds :type "Float (double-precision)") (TriggeredSeconds :type "Float (double-precision)") (InputAction :type "InputAction Object Reference" :default "/Game/Radwa/Inputs/IA_MoveLeftRight.IA_MoveLeftRight"))
  (bind (_returnvalue_x _returnvalue_y) (`KismetMathLibrary.BreakVector` (`self.K2_GetActorLocation`)))
  (:`Triggered`
    (if (`|EnumEquality` (`/Game/Radwa/Blueprints/CustomGameMode.TheGameState` (`self.GameModeRef`)) "NewEnumerator5")
      (set `self.Action Value` ActionValue)
      ;[1 1 1] Limit movement to the left
      (if (< _returnvalue_y (* (`self.BorderLimit`) -1.0))
        (if (> (`self.Action Value`) 0.0)
          (`self.K2_AddActorWorldOffset` (`KismetMathLibrary.MakeVector` 0.0 (* (`self.Action Value`) (`self.PaddleSpeed`))) :!label _label))
        (else
          ;[1 1 1] Limit movement  to the right
          (if (> _returnvalue_y (`self.BorderLimit`))
            (if (< (`self.Action Value`) 0.0)
              (goto _label))
            (else
              (goto _label))))))))

(fn `DecrementLives`
  (if (>= (`self.BallLives`) 0)
    (`/Engine/EditorBlueprintResources/StandardMacros.DecrementInt` (`self.BallLives`))
    (else
      (`KismetSystemLibrary.PrintString` "You're Dead!"))))

(fn `SetBorderLimitRelativeToMeshScale`
  (bind (_returnvalue_x _returnvalue_y) (`KismetMathLibrary.BreakVector` (`SceneComponent.K2_GetComponentScale` (`self.StaticMesh`))))
  (set `self.BorderLimit` (+ (* _returnvalue_y -50.0) 785.0)))

(fn `UserConstructionScript`)